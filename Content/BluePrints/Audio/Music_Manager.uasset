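; Music manager Blueprint that switches the game's background tracks between level 1, level 3 and the DumbleDoor win.
; BeginPlay starts the level 1 track on MusicPart1 after a short delay, and Stoplvl1music halts it.
; Level3Tunes and BeatDumbleDoor swap the boss and win tracks on MusicPart3, calling Play then FadeIn.
; Stoplvl1music calls Stop before FadeOut, so the music cuts immediately.
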(event Custom|Stop%20lvl%201%20music
  (bind _music_part_1 (Variables|Default|Getmusic%20Part%201))
  (Audio|Components|Audio|Stop _music_part_1)
  (Audio|Components|Audio|FadeOut _music_part_1 4.0 0.0 "Linear" :!class /Script/Engine.AudioComponent))

(event Custom|Level%203%20Tunes
  (bind _music_part_3 (Variables|Default|Getmusic%20Part%203))
  (Audio|Components|Audio|SetSound _music_part_3 "/Game/BluePrints/Audio/Music/moc_boss_v3.moc_boss_v3")
  (Audio|Components|Audio|Play _music_part_3 0.0)
  (Audio|Components|Audio|FadeIn _music_part_3 0.5 1.0 0.0 "Linear" :!class /Script/Engine.AudioComponent))

(event Custom|Beat%20DumbleDoor
  (bind _music_part_3 (Variables|Default|Getmusic%20Part%203))
  (Audio|Components|Audio|Stop (Variables|Default|Getmusic%20Part%203))
  (Audio|Components|Audio|SetSound _music_part_3 "/Game/BluePrints/Audio/Music/BassWin.BassWin")
  (Audio|Components|Audio|Play _music_part_3 0.0)
  (Audio|Components|Audio|FadeIn _music_part_3 0.5 1.0 0.0 "Linear" :!class /Script/Engine.AudioComponent))

(event EventBeginPlay
  (bind _music_part_1 (Variables|Default|Getmusic%20Part%201))
  (Utilities|FlowControl|Delay 0.4)
  (Audio|Components|Audio|SetSound _music_part_1 "/Game/BluePrints/Audio/Music/MOC_MX1_v2.MOC_MX1_v2")
  (Audio|Components|Audio|Play _music_part_1 0.0))

(event Collision|EventActorBeginOverlap
  (params (OtherActor :type Actor%20Object%20Reference)))

(event EventTick
  (params (DeltaSeconds :type Float%20%28single-precision%29)))

(fn ConstructionScript)