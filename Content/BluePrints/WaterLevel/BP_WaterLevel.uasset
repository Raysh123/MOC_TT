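; BP_WaterLevel is a rising water volume that punishes the first-person character for touching it.
; DamBurst switches on a timed raise, during which Tick lifts the actor's Z by a fixed step each frame, so the rise is frame-rate dependent.
; Overlapping its Box respawns the character and then calls TakeDamage on it.
; The player reference cached at BeginPlay is unused in these graphs.
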(event OnComponentBeginOverlap(Box)
  (params (OverlappedComponent :type Primitive%20Component%20Object%20Reference) (OtherActor :type Actor%20Object%20Reference) (OtherComp :type Primitive%20Component%20Object%20Reference) (OtherBodyIndex :type Integer) (bFromSweep :type Boolean) (SweepResult :type Hit%20Result%20Structure%20%28by%20ref%29))
  (bind _asbp_first_person_character (Utilities|Casting|CastToBP_FirstPersonCharacter OtherActor))
  (Default|Respawn _asbp_first_person_character)
  (Default|TakeDamage _asbp_first_person_character))

(event Custom|Add%20water%20Level
  (params (B :type Float%20%28double-precision%29))
  (bind _self self)
  (Transformation|SetActorLocation _self (Math|Vector|MakeVector 0.0 0.0 (+ (Variables|Default|GetCurrentWaterLevel _self) B)) false false))

(event Custom|DamBurst
  (Variables|Default|SetRAISE true)
  (Utilities|FlowControl|Delay 26.0)
  (Variables|Default|SetRAISE false))

(event EventBeginPlay
  (bind _asbp_first_person_character (Utilities|Casting|CastToBP_FirstPersonCharacter (Game|Player|GetPlayerPawn 0)))
  (Variables|Default|SetPlayer_Object _asbp_first_person_character))

(event EventTick
  (params (DeltaSeconds :type Float%20%28single-precision%29))
  (Variables|Default|SetCurrentWaterLevel (.z (Transformation|GetActorLocation self)))
  (if (Variables|Default|GetRAISE)
    (CallFunction|AddWaterLevel 2.0)))

(fn ConstructionScript)