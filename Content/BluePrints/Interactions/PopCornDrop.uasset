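; Popcorn-dropping interactable that turns from Happy to Sad for seven seconds when a blue spell overlaps it.
; The hit adds score, raises BP_WaterLevel, plays a pop and random crying sound, and spawns sweet or salty popcorn at random from its arrow.
; Tick sets the face sprites and corn visibility from the current state, and only the Happy state responds to hits.
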(event Custom|ChangeState
  (bind _arrow (Variables|Default|GetArrow))
  (Default|AddScore (Variables|Default|GetPlayerCharacter) 1)
  (Variables|Default|SetState "NewEnumerator1")
  (bind _returnvalue (Actor|GetActorOfClass "/Game/BluePrints/WaterLevel/BP_WaterLevel.BP_WaterLevel_C"))
  (Default|AddWaterLevel _returnvalue 1e+01)
  (Audio|PlaySound2D "/Game/Sound/Balloon_Pop_4.Balloon_Pop_4" 1.0 1.0 0.0 0 0)
  (switch int (Math|Random|RandomIntegerinRange 0 1)
    (:0
      (Game|SpawnActorfromClass "/Game/FirstPerson/Blueprints/BP_PopcornSweet.BP_PopcornSweet_C" (Math|Transform|MakeTransform (.location (Transformation|GetWorldTransform _arrow)) "0, 0, 0" "1.300000,1.300000,1.300000") "Undefined" "MultiplyWithRoot" 0 0))
    (:1
      (Game|SpawnActorfromClass "/Game/FirstPerson/Blueprints/BP_PopcornSalty.BP_PopcornSalty_C" (Math|Transform|MakeTransform (.location (Transformation|GetWorldTransform _arrow)) "0, 0, 0" "1.300000,1.300000,1.300000") "Undefined" "MultiplyWithRoot" 0 0)))
  (Audio|PlaySoundatLocation (.OutItem (Utilities|Array|Random (Utilities|Array|MakeArray "/Game/BluePrints/Audio/Crying_sounds/Crying/Crying_01-01.Crying_01-01" "/Game/BluePrints/Audio/Crying_sounds/Crying/Crying_02-02.Crying_02-02" "/Game/BluePrints/Audio/Crying_sounds/Crying/Crying_02-03.Crying_02-03" "/Game/BluePrints/Audio/Crying_sounds/Crying/Crying_03-01.Crying_03-01" "/Game/BluePrints/Audio/Crying_sounds/Crying/Crying_04-02.Crying_04-02" "/Game/BluePrints/Audio/Crying_sounds/Crying/Crying_05-02.Crying_05-02" "/Game/BluePrints/Audio/Crying_sounds/Crying/Crying_05-06.Crying_05-06" "/Game/BluePrints/Audio/Crying_sounds/Crying/Crying_06-02.Crying_06-02"))) (Transformation|GetActorLocation) "0, 0, 0" 1.0 1.0 0.0 0 0 0 0)
  (Utilities|FlowControl|Delay 7.0)
  (Variables|Default|SetState "NewEnumerator0"))

(event Collision|EventActorBeginOverlap
  (params (OtherActor :type Actor%20Object%20Reference))
  (switch Utilities|FlowControl|Switch|SwitchonCharacterState (Variables|Default|GetState)
    (:NewEnumerator0
      (Utilities|Casting|CastToNS_BlueSpell OtherActor)
      (CallFunction|ChangeState))))

(event EventBeginPlay
  (Variables|Default|SetState "NewEnumerator0")
  (Variables|Default|SetcanInteract false)
  (CallFunction|GetPlayer))

(event EventTick
  (params (DeltaSeconds :type Float%20%28single-precision%29))
  (switch Utilities|FlowControl|Switch|SwitchonCharacterState (Variables|Default|GetState)
    (:NewEnumerator0
      (CallFunction|HappyState))
    (:NewEnumerator1
      (CallFunction|SadState))))

(fn ConstructionScript)

(fn HappyState
  (Rendering|SetVisibility (Variables|Default|GetPaperSprites) true false)
  (Rendering|SetVisibility (Variables|Default|GetPaperSprites1) false false)
  (Rendering|SetVisibility (Variables|Default|GetCorn) true false))

(fn SadState
  (Rendering|SetVisibility (Variables|Default|GetPaperSprites) false false)
  (Rendering|SetVisibility (Variables|Default|GetPaperSprites1) true false)
  (Rendering|SetVisibility (Variables|Default|GetCorn) false false))

(fn GetPlayer
  (bind _asbp_first_person_character (Utilities|Casting|CastToBP_FirstPersonCharacter (Game|Player|GetPlayerPawn 0)))
  (Variables|Default|SetPlayerCharacter _asbp_first_person_character))