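; Spawner actor that repeatedly spawns an actor of a configurable class, intended as enemies, at random points.
; On BeginPlay it starts a looping timer at the SpawnTime interval and caches the world locations of its eight Arrow components into an array.
; Each timer tick spawns at a random cached location, using the spawner's own rotation and scale rather than the arrow's.
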(event Custom|Spawn%20Enemy
  (bind _returnvalue (Transformation|GetActorTransform))
  (Game|SpawnActorfromClass (Variables|Default|GetSpawn%20Actor) (Math|Transform|MakeTransform (.OutItem (Utilities|Array|Random (Variables|Default|GetTransformArrays))) (.rotation _returnvalue) (.scale _returnvalue)) "Undefined" "MultiplyWithRoot" 0 0))

(event EventBeginPlay
  (Utilities|Time|SetTimerbyEvent (delegate Custom|Spawn%20Enemy) (Variables|Default|GetSpawn%20time) true)
  (CallFunction|SetSpawnPoints))

(fn ConstructionScript)

(fn SetSpawnPoints
  (bind _output_get (Variables|Default|SetarrowTF (Transformation|GetWorldLocation (Variables|Default|GetArrow))))
  (bind _output_get_2 (Variables|Default|Setarraow1TF (Transformation|GetWorldLocation (Variables|Default|GetArrow1))))
  (bind _output_get_3 (Variables|Default|Setarrow2TF (Transformation|GetWorldLocation (Variables|Default|GetArrow2))))
  (bind _output_get_4 (Variables|Default|SetArrow3TF (Transformation|GetWorldLocation (Variables|Default|GetArrow3))))
  (bind _output_get_5 (Variables|Default|SetArrow4TF (Transformation|GetWorldLocation (Variables|Default|GetArrow4))))
  (bind _output_get_6 (Variables|Default|SetArrow5TF (Transformation|GetWorldLocation (Variables|Default|GetArrow5))))
  (bind _output_get_7 (Variables|Default|SetArrow6TF (Transformation|GetWorldLocation (Variables|Default|GetArrow6))))
  (bind _output_get_8 (Variables|Default|SetArrow7TF (Transformation|GetWorldLocation (Variables|Default|GetArrow7))))
  (Variables|Default|SetTransformArrays (Utilities|Array|MakeArray _output_get_3 _output_get_2 _output_get _output_get_4 _output_get_5 _output_get_6 _output_get_7 _output_get_8)))