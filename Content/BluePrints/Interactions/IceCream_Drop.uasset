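; Interaction actor with a randomly flavoured ice cream and happy/sad sprites, which drops its cone when hit by a spell.
; A Happy/Sad state drives sprite and cone visibility every Tick.
; An NS_Spell overlap while Happy adds score, raises the water level, pops a sound and spawns BP_PickupIceCream, then destroys the actor after a delay.
; Materials go to the first pickup found by class lookup, not necessarily the spawned one.
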(event Custom|ChangeState
  (Default|AddScore (Variables|Default|GetPlayerCharacter) 1)
  (Variables|Default|SetState "NewEnumerator1"))

(event Collision|EventActorBeginOverlap
  (params (OtherActor :type Actor%20Object%20Reference))
  (switch Utilities|FlowControl|Switch|SwitchonCharacterState (Variables|Default|GetState)
    (:NewEnumerator0
      (Utilities|Casting|CastToNS_Spell OtherActor)
      (CallFunction|ChangeState)
      (bind _returnvalue (Actor|GetActorOfClass "/Game/BluePrints/WaterLevel/BP_WaterLevel.BP_WaterLevel_C"))
      (Default|AddWaterLevel _returnvalue 1e+01)
      (Audio|PlaySound2D "/Game/Sound/Balloon_Pop_4.Balloon_Pop_4" 1.0 1.0 0.0 0 0)
      (bind _returnvalue_2 (Game|SpawnActorfromClass "/Game/FirstPerson/Blueprints/BP_PickupIceCream.BP_PickupIceCream_C" (Math|Transform|MakeTransform (.location (Transformation|GetWorldTransform (Variables|Default|GetCone))) "0, 0, 0" "1.000000,1.000000,1.000000") "Undefined" "MultiplyWithRoot" 0 0))
      (bind _returnvalue_3 (Actor|GetActorOfClass (Utilities|GetClass _returnvalue_2)))
      (Default|AssignMaterials _returnvalue_3 "/Game/Materials/Cone.Cone" (Variables|Default|GetScoop1Mat) (Variables|Default|GetScoop2Mat))
      (Utilities|FlowControl|Delay 5.0)
      (Actor|DestroyActor))))

(event EventBeginPlay
  (Variables|Default|SetState "NewEnumerator0")
  (Variables|Default|SetcanInteract false)
  (CallFunction|GetPlayer)
  (CallFunction|SetMaterials))

(event EventTick
  (params (DeltaSeconds :type Float%20%28single-precision%29))
  (switch Utilities|FlowControl|Switch|SwitchonCharacterState (Variables|Default|GetState)
    (:NewEnumerator0
      (CallFunction|HappyState))
    (:NewEnumerator1
      (CallFunction|SadState))))

(fn ConstructionScript)

(fn HappyState
  (Rendering|SetVisibility (Variables|Default|GetPaperSprites) true false)
  (Rendering|SetVisibility (Variables|Default|GetPaperSprites1) false false))

(fn SadState
  (Rendering|SetVisibility (Variables|Default|GetPaperSprites) false false)
  (Rendering|SetVisibility (Variables|Default|GetPaperSprites1) true false)
  (Rendering|SetVisibility (Variables|Default|GetCone) false false))

(fn GetPlayer
  (bind _asbp_first_person_character (Utilities|Casting|CastToBP_FirstPersonCharacter (Game|Player|GetPlayerPawn 0)))
  (Variables|Default|SetPlayerCharacter _asbp_first_person_character))

(fn SetMaterials
  (bind _output_get (Variables|Default|SetVanilla "/Game/Materials/Vanilla.Vanilla"))
  (bind _output_get_2 (Variables|Default|SetChocolate "/Game/Materials/Chocolate.Chocolate"))
  (bind _output_get_3 (Variables|Default|SetStrawBerry "/Game/Materials/StrawBerry.StrawBerry"))
  (Rendering|Material|SetMaterial (Variables|Default|GetCone) 0 "/Game/Materials/Cone.Cone")
  (bind _output_get_4 (Variables|Default|SetScoop1Mat (.OutItem (Utilities|Array|Random (Utilities|Array|MakeArray _output_get _output_get_2 _output_get_3)))))
  (Rendering|Material|SetMaterial (Variables|Default|GetScoop1) 0 _output_get_4)
  (bind _output_get_5 (Variables|Default|SetScoop2Mat (.OutItem (Utilities|Array|Random (Utilities|Array|MakeArray _output_get _output_get_2 _output_get_3)))))
  (Rendering|Material|SetMaterial (Variables|Default|GetScoop2) 0 _output_get_5))