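; SalaryMan is an NPC that walks forward while Happy until a BP_PickupIceCream overlaps it.
; That overlap adds a player score point, raises BP_WaterLevel, plays a pop sound and switches it to Sad, where it stops moving.
; Each tick, the angle to the player and a right-vector dot product pick one of four directional visuals, idle or creamed by state, shown by toggling component visibility.
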(event Custom|ChangeState
  (Default|AddScore (Variables|Default|GetPlayerCharacter) 1)
  (Variables|Default|SetState "NewEnumerator1"))

(event Custom|ShowRightCreamed
  ;[0.15 0.15 0.15 0.5] Show side
  (Rendering|SetVisibility (Variables|Default|GetFront%20_Idle) false false)
  (Rendering|SetVisibility (Variables|Default|GetBack_Idle) false false)
  (Rendering|SetVisibility (Variables|Default|GetLeft_Idle) false false)
  (Rendering|SetVisibility (Variables|Default|GetRight_Idle) false false)
  (Rendering|SetVisibility (Variables|Default|GetFront%20_Creamed) false false)
  (Rendering|SetVisibility (Variables|Default|GetBack_Creamed) false false)
  (Rendering|SetVisibility (Variables|Default|GetLeft_Creamed) false false)
  (Rendering|SetVisibility (Variables|Default|GetRight_Creamed) true false))

(event Custom|ShowFrontCreamed
  ;[0.15 0.15 0.15 0.5] Show side
  (Rendering|SetVisibility (Variables|Default|GetFront%20_Idle) false false)
  (Rendering|SetVisibility (Variables|Default|GetBack_Idle) false false)
  (Rendering|SetVisibility (Variables|Default|GetLeft_Idle) false false)
  (Rendering|SetVisibility (Variables|Default|GetRight_Idle) false false)
  (Rendering|SetVisibility (Variables|Default|GetFront%20_Creamed) true false)
  (Rendering|SetVisibility (Variables|Default|GetBack_Creamed) false false)
  (Rendering|SetVisibility (Variables|Default|GetLeft_Creamed) false false)
  (Rendering|SetVisibility (Variables|Default|GetRight_Creamed) false false))

(event Custom|Show%20Front
  ;[0.15 0.15 0.15 0.5] Show side
  (Rendering|SetVisibility (Variables|Default|GetFront%20_Idle) true false)
  (Rendering|SetVisibility (Variables|Default|GetBack_Idle) false false)
  (Rendering|SetVisibility (Variables|Default|GetLeft_Idle) false false)
  (Rendering|SetVisibility (Variables|Default|GetRight_Idle) false false)
  (Rendering|SetVisibility (Variables|Default|GetFront%20_Creamed) false false)
  (Rendering|SetVisibility (Variables|Default|GetBack_Creamed) false false)
  (Rendering|SetVisibility (Variables|Default|GetLeft_Creamed) false false)
  (Rendering|SetVisibility (Variables|Default|GetRight_Creamed) false false))

(event Custom|ShowBackCreamed
  ;[0.15 0.15 0.15 0.5] Show side
  (Rendering|SetVisibility (Variables|Default|GetFront%20_Idle) false false)
  (Rendering|SetVisibility (Variables|Default|GetBack_Idle) false false)
  (Rendering|SetVisibility (Variables|Default|GetLeft_Idle) false false)
  (Rendering|SetVisibility (Variables|Default|GetRight_Idle) false false)
  (Rendering|SetVisibility (Variables|Default|GetFront%20_Creamed) false false)
  (Rendering|SetVisibility (Variables|Default|GetBack_Creamed) true false)
  (Rendering|SetVisibility (Variables|Default|GetLeft_Creamed) false false)
  (Rendering|SetVisibility (Variables|Default|GetRight_Creamed) false false))

(event Custom|ShowBack
  ;[0.15 0.15 0.15 0.5] Show side
  (Rendering|SetVisibility (Variables|Default|GetFront%20_Idle) false false)
  (Rendering|SetVisibility (Variables|Default|GetBack_Idle) true false)
  (Rendering|SetVisibility (Variables|Default|GetLeft_Idle) false false)
  (Rendering|SetVisibility (Variables|Default|GetRight_Idle) false false)
  (Rendering|SetVisibility (Variables|Default|GetFront%20_Creamed) false false)
  (Rendering|SetVisibility (Variables|Default|GetBack_Creamed) false false)
  (Rendering|SetVisibility (Variables|Default|GetLeft_Creamed) false false)
  (Rendering|SetVisibility (Variables|Default|GetRight_Creamed) false false))

(event Custom|ShowLeftCreamed
  ;[0.15 0.15 0.15 0.5] Show side
  (Rendering|SetVisibility (Variables|Default|GetFront%20_Idle) false false)
  (Rendering|SetVisibility (Variables|Default|GetBack_Idle) false false)
  (Rendering|SetVisibility (Variables|Default|GetLeft_Idle) false false)
  (Rendering|SetVisibility (Variables|Default|GetRight_Idle) false false)
  (Rendering|SetVisibility (Variables|Default|GetFront%20_Creamed) false false)
  (Rendering|SetVisibility (Variables|Default|GetBack_Creamed) false false)
  (Rendering|SetVisibility (Variables|Default|GetLeft_Creamed) true false)
  (Rendering|SetVisibility (Variables|Default|GetRight_Creamed) false false))

(event Custom|ShowLeft
  ;[0.15 0.15 0.15 0.5] Show side
  (Rendering|SetVisibility (Variables|Default|GetFront%20_Idle) false false)
  (Rendering|SetVisibility (Variables|Default|GetBack_Idle) false false)
  (Rendering|SetVisibility (Variables|Default|GetLeft_Idle) true false)
  (Rendering|SetVisibility (Variables|Default|GetRight_Idle) false false)
  (Rendering|SetVisibility (Variables|Default|GetFront%20_Creamed) false false)
  (Rendering|SetVisibility (Variables|Default|GetBack_Creamed) false false)
  (Rendering|SetVisibility (Variables|Default|GetLeft_Creamed) false false)
  (Rendering|SetVisibility (Variables|Default|GetRight_Creamed) false false))

(event Custom|ShowRight
  ;[0.15 0.15 0.15 0.5] Show side
  (Rendering|SetVisibility (Variables|Default|GetFront%20_Idle) false false)
  (Rendering|SetVisibility (Variables|Default|GetBack_Idle) false false)
  (Rendering|SetVisibility (Variables|Default|GetLeft_Idle) false false)
  (Rendering|SetVisibility (Variables|Default|GetRight_Idle) true false)
  (Rendering|SetVisibility (Variables|Default|GetFront%20_Creamed) false false)
  (Rendering|SetVisibility (Variables|Default|GetBack_Creamed) false false)
  (Rendering|SetVisibility (Variables|Default|GetLeft_Creamed) false false)
  (Rendering|SetVisibility (Variables|Default|GetRight_Creamed) false false))

(event Collision|EventActorBeginOverlap
  (params (OtherActor :type Actor%20Object%20Reference))
  (switch Utilities|FlowControl|Switch|SwitchonCharacterState (Variables|Default|GetState)
    (:NewEnumerator0
      (Utilities|Casting|CastToBP_PickupIceCream OtherActor)
      (CallFunction|ChangeState)
      (bind _returnvalue (Actor|GetActorOfClass "/Game/BluePrints/WaterLevel/BP_WaterLevel.BP_WaterLevel_C"))
      (Default|AddWaterLevel _returnvalue 1e+01)
      (Audio|PlaySound2D "/Game/Sound/Balloon_Pop_4.Balloon_Pop_4" 1.0 1.0 0.0 0 0))))

(event EventBeginPlay
  (Variables|Default|SetState "NewEnumerator0")
  (Variables|Default|SetcanInteract false)
  (CallFunction|GetPlayer))

(event EventTick
  (params (DeltaSeconds :type Float%20%28single-precision%29))
  (switch Utilities|FlowControl|Switch|SwitchonCharacterState (Variables|Default|GetState)
    (:NewEnumerator0
      (CallFunction|HappyState)
      (CallFunction|FaceDirection))
    (:NewEnumerator1
      (CallFunction|SadState)
      (CallFunction|FaceDirectionCreamed))))

(fn ConstructionScript)

(fn HappyState
  (Transformation|AddActorLocalOffset "3.000000,0.000000,0.000000" false false))

(fn SadState)

(fn GetPlayer
  (bind _asbp_first_person_character (Utilities|Casting|CastToBP_FirstPersonCharacter (Game|Player|GetPlayerPawn 0)))
  (Variables|Default|SetPlayerCharacter _asbp_first_person_character))

(fn AngletoPlayer
  (Variables|Default|SetAngle (Class|KismetMathLibrary|DegAcos (Math|Vector|DotProduct (Math|Vector|Normalize (Math|Vector|GetForwardVector (Transformation|GetActorRotation))) (Math|Vector|Normalize (- (Transformation|GetActorLocation (Game|Player|GetPlayerPawn 0)) (Transformation|GetActorLocation)))))))

(fn RightorLeft
  (Variables|Default|SetOnRight (> (Math|Vector|DotProduct (Transformation|GetActorRightVector) (- (Transformation|GetActorLocation (Game|Player|GetPlayerPawn 0)) (Transformation|GetActorLocation))) 0.0)))

(fn FaceDirection
  (CallFunction|AngletoPlayer)
  (CallFunction|RightorLeft)
  (if (<= (Variables|Default|GetAngle) 45.0)
    (CallFunction|ShowFront)
    (elif (> (Variables|Default|GetAngle) 135.0)
      (CallFunction|ShowBack)
      (elif (Variables|Default|GetOnRight)
        (CallFunction|ShowRight)
        (else
          (CallFunction|ShowLeft))))))

(fn FaceDirectionCreamed
  (CallFunction|AngletoPlayer)
  (CallFunction|RightorLeft)
  (if (<= (Variables|Default|GetAngle) 45.0)
    (CallFunction|ShowFrontCreamed)
    (elif (> (Variables|Default|GetAngle) 135.0)
      (CallFunction|ShowBackCreamed)
      (elif (Variables|Default|GetOnRight)
        (CallFunction|ShowRightCreamed)
        (else
          (CallFunction|ShowLeftCreamed))))))