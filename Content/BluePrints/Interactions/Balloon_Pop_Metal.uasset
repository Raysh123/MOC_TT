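; Floating balloon target that pops when a BP_PickupBase actor overlaps it, scoring for the player and raising the water level.
; A Happy/Sad state drives Tick: Happy drifts the actor along local Y, while Sad swaps the paper sprite and hides both balloons.
; Overlap sets Sad, updates the first-person character and BP_WaterLevel, and plays a pop sound.
; A Delay on the Happy branch destroys the actor after a fixed lifetime.
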(event Custom|ChangeState
  (Default|AddScore (Variables|Default|GetPlayerCharacter) 1)
  (Variables|Default|SetState "NewEnumerator1"))

(event Collision|EventActorBeginOverlap
  (params (OtherActor :type Actor%20Object%20Reference))
  (Utilities|Casting|CastToBP_PickupBase OtherActor)
  (CallFunction|ChangeState)
  (bind _returnvalue (Actor|GetActorOfClass "/Game/BluePrints/WaterLevel/BP_WaterLevel.BP_WaterLevel_C"))
  (Default|AddWaterLevel _returnvalue 1e+01)
  (Audio|PlaySound2D "/Game/Sound/Balloon_Pop_4.Balloon_Pop_4" 1.0 1.0 0.0 0 0))

(event EventBeginPlay
  (Variables|Default|SetState "NewEnumerator0")
  (Variables|Default|SetcanInteract false)
  (CallFunction|GetPlayer))

(event EventTick
  (params (DeltaSeconds :type Float%20%28single-precision%29))
  (switch Utilities|FlowControl|Switch|SwitchonCharacterState (Variables|Default|GetState)
    (:NewEnumerator0
      (CallFunction|HappyState)
      (Utilities|FlowControl|Delay 15.0)
      (Actor|DestroyActor))
    (:NewEnumerator1
      (CallFunction|SadState))))

(fn ConstructionScript)

(fn HappyState
  (Rendering|SetVisibility (Variables|Default|GetPaperSprites) true false)
  (Rendering|SetVisibility (Variables|Default|GetPaperSprites1) false false)
  (Transformation|AddActorLocalOffset "0.000000,3.000000,0.000000" false false))

(fn SadState
  (Rendering|SetVisibility (Variables|Default|GetPaperSprites) false false)
  (Rendering|SetVisibility (Variables|Default|GetPaperSprites1) true false)
  (Rendering|SetVisibility (Variables|Default|GetBalloon) false false))

(fn GetPlayer
  (bind _asbp_first_person_character (Utilities|Casting|CastToBP_FirstPersonCharacter (Game|Player|GetPlayerPawn 0)))
  (Variables|Default|SetPlayerCharacter _asbp_first_person_character))