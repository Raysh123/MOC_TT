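; Theater screen target that cycles flipbook films and reacts to objects thrown into its Box.
; Tick runs a boolean state machine paced by Delays, alternating a tutorial with a random red or green hero film plus random dialogue and music.
; Salty popcorn during hero 1 or sweet during hero 2 stops audio, raises BP_WaterLevel and triggers cracks and villain laughter.
; An Oscar hit bursts the dam and destroys the screen.
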(event OnComponentBeginOverlap(Box)
  (params (OverlappedComponent :type Primitive%20Component%20Object%20Reference) (OtherActor :type Actor%20Object%20Reference) (OtherComp :type Primitive%20Component%20Object%20Reference) (OtherBodyIndex :type Integer) (bFromSweep :type Boolean) (SweepResult :type Hit%20Result%20Structure%20%28by%20ref%29))
  (Utilities|Casting|CastToOscar OtherActor
    (:then
      (Audio|PlaySoundatLocation "/Game/BluePrints/Audio/Sound_Design/FX_Screen_Impact-003.FX_Screen_Impact-003" (Transformation|GetActorLocation) "0, 0, 0" 1.0 1.0 0.0 0 0 0 0)
      (bind _returnvalue (Actor|GetActorOfClass "/Game/BluePrints/WaterLevel/BP_WaterLevel.BP_WaterLevel_C"))
      (Default|DamBurst _returnvalue)
      (Utilities|FlowControl|Delay 0.2)
      (Actor|DestroyActor))
    (:CastFailed
      (if (Variables|Default|GetisHero1)
        (Utilities|Casting|CastToBP_PopcornSalty OtherActor)
        (Audio|PlaySoundatLocation "/Game/BluePrints/Audio/Sound_Design/FX_Screen_Impact-002.FX_Screen_Impact-002" (Transformation|GetActorLocation) "0, 0, 0" 1.0 1.0 0.0 0 0 0 0)
        (bind _returnvalue_2 (Actor|GetActorOfClass "/Game/BluePrints/WaterLevel/BP_WaterLevel.BP_WaterLevel_C"))
        (Default|AddWaterLevel _returnvalue_2 1e+02)
        (Audio|Components|Audio|Stop (Variables|Default|GetMusic))
        (Variables|Default|SetisHero1 false)
        (Variables|Default|SetHurt true)
        (elif (Variables|Default|Getis%20Hero%202)
          (Utilities|Casting|CastToBP_PopcornSweet OtherActor)
          (Audio|PlaySoundatLocation "/Game/BluePrints/Audio/Sound_Design/FX_Screen_Impact-004.FX_Screen_Impact-004" (Transformation|GetActorLocation) "0, 0, 0" 1.0 1.0 0.0 0 0 0 0)
          (bind _returnvalue_3 (Actor|GetActorOfClass "/Game/BluePrints/WaterLevel/BP_WaterLevel.BP_WaterLevel_C"))
          (Default|AddWaterLevel _returnvalue_3 1e+02)
          (Audio|Components|Audio|Stop (Variables|Default|GetMusic))
          (Variables|Default|Setis%20Hero%202 false)
          (Variables|Default|SetHurt true))))))

(event Custom|AddVillainSprites)

(event Custom|Play%20Sound%20Cue
  (bind _dialogue (Variables|Default|GetDialogue))
  (bind _music (Variables|Default|GetMusic))
  (Audio|Components|Audio|SetSound _dialogue (.OutItem (Utilities|Array|Random (Utilities|Array|MakeArray "/Game/BluePrints/Audio/Hero_DX/Hero_DX-03.Hero_DX-03" "/Game/BluePrints/Audio/Hero_DX/Hero_DX-05.Hero_DX-05" "/Game/BluePrints/Audio/Hero_DX/Hero_DX-07.Hero_DX-07" "/Game/BluePrints/Audio/Hero_DX/Hero_DX-09.Hero_DX-09"))))
  (Audio|Components|Audio|Play _dialogue 0.0)
  (Transformation|SetWorldLocation _dialogue (Transformation|GetWorldLocation _dialogue) false false)
  (Audio|Components|Audio|SetSound _music (.OutItem (Utilities|Array|Random (Utilities|Array|MakeArray "/Game/BluePrints/Audio/Music/MOC_action_2_MX.MOC_action_2_MX" "/Game/BluePrints/Audio/Music/MOC_Action_MX_v1.MOC_Action_MX_v1"))))
  (Audio|Components|Audio|Play _music 0.0)
  (Transformation|SetWorldLocation _music (Transformation|GetWorldLocation _music) false false))

(event Custom|Reset
  (Variables|Default|SetHurt true)
  (Variables|Default|Setis%20Hero%202 false)
  (Variables|Default|SetisHero1 false)
  (Variables|Default|SetisIdle false))

(event EventBeginPlay)

(event EventTick
  (params (DeltaSeconds :type Float%20%28single-precision%29))
  (if (Variables|Default|GetisIdle)
    (Sprite|SetFlipbook (Variables|Default|GetFlipbook) "/Paper2D/Tutorial/Paper2D/TutorialAssets/TutorialFlipBook.TutorialFlipBook")
    (Utilities|FlowControl|Delay 5.0)
    (Variables|Default|SetIntValue (Math|Random|RandomIntegerinRange 0 1))
    (CallFunction|PlaySoundCue)
    (Variables|Default|SetisIdle false)
    (switch int (Variables|Default|GetIntValue)
      (:0
        (Variables|Default|SetisHero1 true)
        (Variables|Default|Setis%20Hero%202 false))
      (:1
        (Variables|Default|Setis%20Hero%202 true)
        (Variables|Default|SetisHero1 false)))
    (elif (Variables|Default|GetisHero1)
      (if (== (Variables|Default|GetIntValue) 0)
        (Sprite|SetFlipbook (Variables|Default|GetFlipbook) "/Game/PicsAndAnimation/Theater/GIF_WithColor/Red_Hero.Red_Hero")
        (Utilities|FlowControl|Delay 4.0)
        (else
          (Sprite|SetFlipbook (Variables|Default|GetFlipbook) "/Game/PicsAndAnimation/Theater/GIF_WithColor/Green/Red_Hero2.Red_Hero2")
          (Utilities|FlowControl|Delay 6.0)))
      (Variables|Default|SetisIdle true)
      (Variables|Default|SetisHero1 false)
      (elif (Variables|Default|Getis%20Hero%202)
        (if (== (Variables|Default|GetIntValue) 0)
          (Sprite|SetFlipbook (Variables|Default|GetFlipbook) "/Game/PicsAndAnimation/Theater/GIF_WithColor/Green/Green_HEro2.Green_HEro2")
          (Utilities|FlowControl|Delay 5.0)
          (else
            (Sprite|SetFlipbook (Variables|Default|GetFlipbook) "/Game/PicsAndAnimation/Theater/GIF_WithColor/Green/GreenHero.GreenHero")
            (Utilities|FlowControl|Delay 3.0)))
        (Variables|Default|SetisIdle true)
        (Variables|Default|Setis%20Hero%202 false)
        (elif (Variables|Default|GetHurt)
          (Sprite|SetFlipbook (Variables|Default|GetFlipbook) "/Game/BluePrints/Theater/Projectile/Cracks.Cracks")
          (Sprite|SetFlipbook (Variables|Default|GetFlipbook1) "/Game/PicsAndAnimation/Theater/Villain/Laugh/Evil_Laugh.Evil_Laugh")
          (Utilities|FlowControl|Delay 3.0)
          (Variables|Default|SetHurt false)
          (Variables|Default|SetisIdle true)
          (if (== (Variables|Default|GetIntValue) 0)
            (Sprite|SetFlipbook (Variables|Default|GetFlipbook1) "/Game/PicsAndAnimation/Theater/Villain/1/Villain.Villain")
            (else
              (Sprite|SetFlipbook (Variables|Default|GetFlipbook1) "/Game/PicsAndAnimation/Theater/Villain/3/Villain3.Villain3"))))))))

(fn ConstructionScript)